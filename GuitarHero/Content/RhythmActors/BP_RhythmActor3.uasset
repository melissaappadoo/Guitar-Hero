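; BP_RhythmActor3 is a rhythm actor that travels along Lane3 of the level's BP_RhythmLanes actor.
; On BeginPlay it finds and caches the lanes actor, then starts a timeline with play rate scaled by TimeToCompleteSeconds.
; Each update lerps spline distance from the lane's end back to its start, setting world-space location and local-space spline rotation.
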(event Custom|Move%20Object
  (bind _rhythmlane (Variables|Default|GetRhythmLane))
  (bind _lane_3 (Variables|/Game/BP_RhythmLanes.BP_RhythmLanes_C|GetLane%203 _rhythmlane))
  ;[1 1 1] Moves Actor on Spline
  (Components|Timeline|SetPlayRate (Variables|Default|GetT%20Move%20Object) (/ 1.0 (Variables|Default|GetTime%20To%20Complete%20%28seconds%29)))
  (bind _move_track (Timeline|T%20Move%20Object Play)
    (:Update
      (Transformation|SetActorTransform (Math|Transform|MakeTransform (Spline|GetLocationatDistanceAlongSpline _lane_3 (Math|Float|Lerp (Spline|GetSplineLength (Variables|/Game/BP_RhythmLanes.BP_RhythmLanes_C|GetLane%203 (Variables|Default|GetRhythmLane))) 0.0 _move_track) "World") (Spline|GetRotationatDistanceAlongSpline _lane_3 (Math|Float|Lerp (Spline|GetSplineLength (Variables|/Game/BP_RhythmLanes.BP_RhythmLanes_C|GetLane%203 (Variables|Default|GetRhythmLane))) 0.0 _move_track) "Local") "1.000000,1.000000,1.000000")))))

(event EventBeginPlay
  (bind _returnvalue (Actor|GetActorOfClass "/Game/BP_RhythmLanes.BP_RhythmLanes_C"))
  (Variables|Default|SetRhythmLane _returnvalue)
  (CallFunction|MoveObject))

(fn ConstructionScript)