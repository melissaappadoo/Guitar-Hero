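; Three-lane rhythm game actor that maps the A, S and D Enhanced Input actions to note judgement boxes.
; A press scores when that lane's note class overlaps its box, flashing the lane plane and printing random praise; otherwise it prints a miss.
; Only lane A tracks a streak, doubling the entire score on each hit from ten onward.
; Destroyer volumes remove any actor that overlaps them.
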(event OnComponentBeginOverlap(Destroyer)
  (params (OverlappedComponent :type Primitive%20Component%20Object%20Reference) (OtherActor :type Actor%20Object%20Reference) (OtherComp :type Primitive%20Component%20Object%20Reference) (OtherBodyIndex :type Integer) (bFromSweep :type Boolean) (SweepResult :type Hit%20Result%20Structure%20%28by%20ref%29))
  ;[1 0 0] Destroy Notes
  (Actor|DestroyActor OtherActor))

(event OnComponentBeginOverlap(Destroyer2)
  (params (OverlappedComponent :type Primitive%20Component%20Object%20Reference) (OtherActor :type Actor%20Object%20Reference) (OtherComp :type Primitive%20Component%20Object%20Reference) (OtherBodyIndex :type Integer) (bFromSweep :type Boolean) (SweepResult :type Hit%20Result%20Structure%20%28by%20ref%29))
  ;[1 0 0] Destroy Notes
  (Actor|DestroyActor OtherActor))

(event OnComponentBeginOverlap(Destroyer3)
  (params (OverlappedComponent :type Primitive%20Component%20Object%20Reference) (OtherActor :type Actor%20Object%20Reference) (OtherComp :type Primitive%20Component%20Object%20Reference) (OtherBodyIndex :type Integer) (bFromSweep :type Boolean) (SweepResult :type Hit%20Result%20Structure%20%28by%20ref%29))
  ;[1 0 0] Destroy Notes
  (Actor|DestroyActor OtherActor))

(event Input|EnhancedActionEvents|EnhancedInputActionIA_A
  (params (ActionValue :type Boolean) (ElapsedSeconds :type Float%20%28double-precision%29) (TriggeredSeconds :type Float%20%28double-precision%29) (InputAction :type Input%20Action%20Object%20Reference :default "/Game/IA_A.IA_A")))

(event Input|EnhancedActionEvents|EnhancedInputActionIA_S
  (params (ActionValue :type Boolean) (ElapsedSeconds :type Float%20%28double-precision%29) (TriggeredSeconds :type Float%20%28double-precision%29) (InputAction :type Input%20Action%20Object%20Reference :default "/Game/IA_S.IA_S"))
  (bind _plane1 (Variables|Default|GetPlane1))
  ;[1 0.9873 0.2104] Target Notes (Hit or Miss?)
  (:Triggered
    (Variables|Default|SetS%20Elapsed%20Seconds ElapsedSeconds)
    (if (== (Utilities|Array|Length (Collision|GetOverlappingActors (Variables|Default|GetRhythmJudgementBox2) "/Game/RhythmActors/BP_RhythmActor2.BP_RhythmActor2_C" :!class /Script/Engine.PrimitiveComponent)) 0)
      (Development|PrintString "Missed!")
      (else
        (Utilities|FlowControl|Sequence
          (:then_0
            (Rendering|Material|SetMaterial _plane1 0 "/Game/StarterContent/Particles/Materials/m_flare_01.m_flare_01")
            (Utilities|FlowControl|Delay 0.1)
            (Rendering|Material|SetMaterial _plane1 0 "/Game/StarterContent/Particles/Materials/M_Burst.M_Burst")
            (Variables|Default|SetScore (+ (Variables|Default|GetScore) 50)))
          (:then_1
            (CallFunction|GoodHit)))))))

(event Input|EnhancedActionEvents|EnhancedInputActionIA_D
  (params (ActionValue :type Boolean) (ElapsedSeconds :type Float%20%28double-precision%29) (TriggeredSeconds :type Float%20%28double-precision%29) (InputAction :type Input%20Action%20Object%20Reference :default "/Game/IA_D.IA_D"))
  (bind _plane2 (Variables|Default|GetPlane2))
  ;[1 0.9873 0.2104] Target Notes (Hit or Miss?)
  (:Triggered
    (Variables|Default|SetD%20Elapsed%20Seconds ElapsedSeconds)
    (if (== (Utilities|Array|Length (Collision|GetOverlappingActors (Variables|Default|GetRhythmJudgementBox3) "/Game/RhythmActors/BP_RhythmActor3.BP_RhythmActor3_C" :!class /Script/Engine.PrimitiveComponent)) 0)
      (Development|PrintString "Missed!")
      (else
        (Utilities|FlowControl|Sequence
          (:then_0
            (Rendering|Material|SetMaterial _plane2 0 "/Game/StarterContent/Particles/Materials/m_flare_01.m_flare_01")
            (Utilities|FlowControl|Delay 0.1)
            (Rendering|Material|SetMaterial _plane2 0 "/Game/StarterContent/Particles/Materials/M_Burst.M_Burst")
            (Variables|Default|SetScore (+ (Variables|Default|GetScore) 50)))
          (:then_1
            (CallFunction|GoodHit)))))))

(event Input|EnhancedActionEvents|EnhancedInputActionIA_A
  (params (ActionValue :type Boolean) (ElapsedSeconds :type Float%20%28double-precision%29) (TriggeredSeconds :type Float%20%28double-precision%29) (InputAction :type Input%20Action%20Object%20Reference :default "/Game/IA_A.IA_A"))
  (bind _plane (Variables|Default|GetPlane))
  ;[1 0.9873 0.2104] Target Notes (Hit or Miss?)
  (:Triggered
    (Variables|Default|SetA%20Elapsed%20Seconds ElapsedSeconds)
    (if (== (Utilities|Array|Length (Collision|GetOverlappingActors (Variables|Default|GetRhythmJudgementBox) "/Game/RhythmActors/BP_RhythmActor.BP_RhythmActor_C" :!class /Script/Engine.PrimitiveComponent)) 0)
      (Development|PrintString "Missed!")
      (Variables|Default|SetOnNoteStreak false)
      (Variables|Default|SetNoteStreak 0)
      (Variables|Default|SetMultiplier false)
      (else
        (Utilities|FlowControl|Sequence
          (:then_0
            (Rendering|Material|SetMaterial _plane 0 "/Game/StarterContent/Particles/Materials/m_flare_01.m_flare_01")
            (Utilities|FlowControl|Delay 0.1)
            (Rendering|Material|SetMaterial _plane 0 "/Game/StarterContent/Particles/Materials/M_Burst.M_Burst")
            (Variables|Default|SetScore (+ (Variables|Default|GetScore) 50))
            (Variables|Default|SetOnNoteStreak true)
            (Variables|Default|SetNoteStreak (+ (Variables|Default|GetNoteStreak) 1))
            (if (>= (Variables|Default|GetNoteStreak) 10)
              (Variables|Default|SetMultiplier true)
              (Variables|Default|SetScore (* (Variables|Default|GetScore) 2))))
          (:then_1
            (CallFunction|GoodHit)))))))

(event EventBeginPlay
  (bind _returnvalue (Game|GetPlayerController 0))
  (bind _returnvalue_2 (PlayerController|LocalPlayerSubsystems|GetEnhancedInputLocalPlayerSubsystem _returnvalue))
  (Class|EnhancedInputSubsystemInterface|ClearAllMappings _returnvalue_2)
  (Input|AddMappingContext _returnvalue_2 "/Game/MC_Keys.MC_Keys" 0 "(bIgnoreAllPressedKeysUntilRelease=True,bForceImmediately=False)")
  (Input|EnableInput _returnvalue)
  (bind _returnvalue_3 (Actor|GetActorOfClass "/Script/LevelSequence.LevelSequenceActor"))
  (Variables|Default|SetL_Drone _returnvalue_3))

(event EventTick
  (params (DeltaSeconds :type Float%20%28single-precision%29)))

(fn ConstructionScript)

(fn GoodHit
  (switch int (Math|Random|RandomIntegerinRange 0 3)
    (:0
      (Development|PrintString "Nice!"))
    (:1
      (Development|PrintString "Great!"))
    (:2
      (Development|PrintString "Excellect!"))
    (:3
      (Development|PrintString "Good!"))))